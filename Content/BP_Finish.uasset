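; BP_Finish is a challenge finish trigger that plays a win sequence when a living PlayerPawn overlaps it.
; A timeline drives the pawn's speed scale, lifts it through its gravity well offset and rolls its mesh.
; When the timeline ends, it sets the ClassicGameMode's next challenge start, destroys the pawn and resets all BP_Popup actors.
; The construction script passes WinText to the SuccessText child popup.
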(event `self.ReceiveBeginPlay`)

(event `self.ReceiveActorBeginOverlap`
  (params (OtherActor :type "Actor Object Reference"))
  (bind _asplayer_pawn (cast `/Game/PlayerPawn` OtherActor))
  (if (not (`/Game/PlayerPawn.Dead` _asplayer_pawn))
    (set `/Game/PlayerPawn.NeedsFloor` false _asplayer_pawn)
    (bind (_direction _flyup _speed) (`Timeline|WinTimeline` :!via `PlayFromStart`)
      (:`Update`
        (set `/Game/PlayerPawn.SpeedScale` _speed _asplayer_pawn)
        (set `/Game/PlayerPawn.GravityWellOffset` (* (0.0 0.0 800.0) _flyup) _asplayer_pawn)
        (bind _playermesh (`/Game/PlayerPawn.PlayerMesh` _asplayer_pawn))
        (bind (_relativerotation_roll _relativerotation_pitch _relativerotation_yaw) (`KismetMathLibrary.BreakRotator` (`SceneComponent.RelativeRotation` _playermesh)))
        (`SceneComponent.K2_SetRelativeRotation` _playermesh (`KismetMathLibrary.MakeRotator` (* _flyup -90.0) _relativerotation_pitch _relativerotation_yaw) false false))
      (:`Finished`
        (bind _asclassic_game_mode (cast `/Game/ClassicGameMode` (`GameplayStatics.GetGameMode`)))
        (set `/Game/ClassicGameMode.CurrentChallengeStart` (`self.NextPlayerStart`) _asclassic_game_mode)
        (`self.K2_DestroyActor` _asplayer_pawn)
        (bind _outactors (`GameplayStatics.GetAllActorsOfClass` "/Game/BP_Popup.BP_Popup_C"))
        (for _array_element _outactors
          (`/Game/BP_Popup.Reset` _array_element))))))

(fn `UserConstructionScript`
  (bind _asbp_finish_popup (cast `/Game/BP_Finish_Popup` (`ChildActorComponent.ChildActor` (`self.SuccessText`))))
  (set `/Game/BP_Finish_Popup.Text` (`self.WinText`) _asbp_finish_popup))