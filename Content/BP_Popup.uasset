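; Popup actor that scales its child components into view when the player pawn overlaps it.
; On BeginPlay, Reset shrinks every child of the root except Box to zero scale.
; An overlap waits for a configurable delay, then plays a timeline that drives the uniform scale of all root children, Box included.
; An Animating flag ignores new overlaps until the timeline finishes, after which another overlap replays it.
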(event `Reset`
  (for _array_element (`SceneComponent.GetChildrenComponents` (`self.DefaultSceneRoot`) false)
    (if (not (== _array_element (`self.Box`)))
      (`SceneComponent.SetRelativeScale3D` _array_element (0.0 0.0 0.0)))))

(event `self.ReceiveBeginPlay`
  (`self.Reset`))

(event `self.ReceiveActorBeginOverlap`
  (params (OtherActor :type "Actor Object Reference"))
  (if (not (`self.Animating`))
    (cast `/Game/PlayerPawn` OtherActor)
    (set `self.Animating` true)
    (`KismetSystemLibrary.Delay` (`self.Delay`))
    (bind (_direction _scale) (`Timeline|ChildrenScaleTimeline` :!via `PlayFromStart`)
      (:`Update`
        (for _array_element (`SceneComponent.GetChildrenComponents` (`self.DefaultSceneRoot`) false)
          (`SceneComponent.SetRelativeScale3D` _array_element (* (1.0 1.0 1.0) _scale))))
      (:`Finished`
        (set `self.Animating` false)))))

(fn `UserConstructionScript`)